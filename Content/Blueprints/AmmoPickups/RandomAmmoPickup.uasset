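; Component that drops a random ammo pickup when its owning Geometry Collection destructible breaks.
; On BeginPlay it binds to the owner's Chaos break event.
; The first break spawns a random class from the AmmoPickups list at the break location, guarded by a spawned-once flag.
; A DoOnce limits the collapse sound to a single play at that location.
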(event Custom|OnChaosBreakEvent_Event
  (params (BreakEvent :type Chaos%20Break%20Event%20Structure%20%28by%20ref%29))
  (bind _location (Utilities|Struct|BreakChaosBreakEvent BreakEvent))
  (CallFunction|SpawnAmmoPickup _location)
  (Utilities|FlowControl|DoOnce false
    (:Completed
      (Audio|PlaySoundatLocation "/Game/StarterContent/Audio/Collapse_Cue.Collapse_Cue" _location "0, 0, 0" 1.0 1.0 0.0 0 0 0 0))))

(event EventBeginPlay
  (bind _output_get (Variables|Default|SetParent%20Destructible (Actor|GetComponentbyClass (Components|GetOwner) "/Script/GeometryCollectionEngine.GeometryCollectionComponent")))
  (EventDispatchers|AssignOnChaosBreakEvent _output_get (delegate Custom|OnChaosBreakEvent_Event)))

(event EventTick
  (params (DeltaSeconds :type Float%20%28single-precision%29)))

(fn SpawnAmmoPickup
  (params (Spawn%20Location :type Vector))
  (if (not (Variables|Default|GetHas%20Spawned%20Once))
    (bind _output_get (LocalVariables|SetChosen%20Pickup (.OutItem (Utilities|Array|Random (Variables|Default|GetAmmo%20Pickups)))))
    (Game|SpawnActorfromClass _output_get (Math|Conversions|ToTransform(Vector) Spawn%20Location) "Undefined" "MultiplyWithRoot" (Components|GetOwner) 0)
    (Variables|Default|SetHas%20Spawned%20Once true)))
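; Actor component that gives a Chaos destructible a hit-point gate before it can break.
; On BeginPlay it finds the owner's Geometry Collection component, disables damage from collision and binds to its begin-overlap event.
; Each overlap by a ShootMePlsProjectile decrements Health, or re-enables collision damage once Health is 1 or lower, leaving the breaking to Chaos.
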(event Custom|OnComponentBeginOverlap_Event
  (params (OverlappedComponent :type Primitive%20Component%20Object%20Reference) (OtherActor :type Actor%20Object%20Reference) (OtherComp :type Primitive%20Component%20Object%20Reference) (OtherBodyIndex :type Integer) (bFromSweep :type Boolean) (SweepResult :type Hit%20Result%20Structure%20%28by%20ref%29))
  (Utilities|Casting|CastToShootMePlsProjectile OtherActor)
  (if (<= (Variables|Default|GetHealth) 1)
    (Class|GeometryCollectionComponent|SetEnableDamagefromCollision (Variables|Default|GetParentDestructible) true)
    (else
      (Math|Integer|DecrementInt (Variables|Default|GetHealth)))))

(event EventBeginPlay
  (bind _output_get (Variables|Default|SetParentDestructible (Actor|GetComponentbyClass (Components|GetOwner) "/Script/GeometryCollectionEngine.GeometryCollectionComponent")))
  (Class|GeometryCollectionComponent|SetEnableDamagefromCollision _output_get false)
  (Collision|AssignOnComponentBeginOverlap (Variables|Default|GetParentDestructible) (delegate Custom|OnComponentBeginOverlap_Event)))

(event EventTick
  (params (DeltaSeconds :type Float%20%28single-precision%29)))